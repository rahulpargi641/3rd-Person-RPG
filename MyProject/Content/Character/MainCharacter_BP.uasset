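; Main character Blueprint that opens the game on a paused menu and offers a key for showing pickup locations.
; On BeginPlay it creates the W_Menu widget, adds it to the viewport and pauses the game.
; Pressing P calls ShowPickupLocations, whose body is not in this graph.
; Health, Stamina and Coins adjustments sit in unconnected nodes that never run, and overlap, tick and construction logic are empty.
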(event `self.ReceiveBeginPlay`
  (bind _returnvalue (`|CreateWidget` "/Game/Blueprints/W_Menu.W_Menu_C"))
  (`UserWidget.AddToViewport` _returnvalue 0)
  (`GameplayStatics.SetGamePaused` true))

(event `Key|P`
  (params (Key :type "Key Structure"))
  (:`Pressed`
    (`self.ShowPickupLocations`)))

(fn `UserConstructionScript`)